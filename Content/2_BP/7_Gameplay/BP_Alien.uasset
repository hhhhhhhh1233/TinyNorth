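; BP_Alien is the Blueprint layer of the player's alien, handling its HUD, pause flow and death screen effect.
; BeginPlay creates the HUD widget and passes it to HudWidget for Angelscript use.
; Escape, Q in editor, or PauseEvent opens a pause menu holding a back-reference to the alien, switching input mode and centering the cursor.
; Unpause restores gameplay, while PlayDeathHudEffect triggers a HUD fade out and in.
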(event EventBeginPlay
  (|CallParentFunction)
  (bind _returnvalue (UserInterface|CreateWidget "/Game/2_BP/6_UI/HUD/WBP_HUD.WBP_HUD_C"))
  (UserInterface|Viewport|AddtoViewport _returnvalue 0)
  (bind _output_get (Variables|Default|SetHUD _returnvalue))
  ;[0.15 0.15 0.15 0.5] Set the reference for angelscript
  (Variables|Default|SetHudWidget _output_get)
  (Variables|Default|SetPaused false))

(event Collision|EventActorBeginOverlap
  (params (OtherActor :type Actor%20Object%20Reference)))

(event EventPauseEvent
  (CallFunction|Pause))

(event EventTick
  (params (DeltaSeconds :type Float%20%28single-precision%29))
  (|CallParentFunction DeltaSeconds))

(event EventPlayDeathHudEffect
  (params (FadeTime :type Float%20%28double-precision%29))
  ;[0.15 0.15 0.15 0.5] When Player Dies
  (Default|StartFadeOutandin (Variables|Default|GetHUD) FadeTime))

(event Input|KeyboardEvents|Escape
  (params (Key :type Key%20Structure :default "None"))
  (:Pressed
    (CallFunction|Pause)))

(event Input|KeyboardEvents|Q
  (params (Key :type Key%20Structure :default "None"))
  (:Pressed
    (bind _returnvalue (Class|ModuleMiscMiscStatics|IsEditor))
    (if _returnvalue
      (CallFunction|Pause))))

(fn ConstructionScript
  (|CallParentFunction))

(fn Unpause
  (if (Variables|Default|GetPaused)
    (Variables|Default|SetPaused false)
    (Widget|SetVisibility (Variables|Default|GetHUD) "Visible")
    (Input|SetInputModeGameOnly (Class|GameplayStatics|GetPlayerControllerfromID) false)
    (Variables|/Script/Engine.PlayerController|SetbShowMouseCursor (Class|GameplayStatics|GetPlayerControllerfromID) (Variables|Default|GetPaused))
    (Game|SetGamePaused false)))

(fn Pause
  (if (not (Variables|Default|GetPaused))
    (Variables|Default|SetPaused true)
    (Widget|SetVisibility (Variables|Default|GetHUD) "Hidden")
    (bind _returnvalue (UserInterface|CreateWidget "/Game/2_BP/6_UI/PauseMenu/WBP_PauseMenu.WBP_PauseMenu_C"))
    (UserInterface|Viewport|AddtoViewport _returnvalue 0)
    (bind _output_get (Variables|Default|SetPauseMenu _returnvalue))
    (Variables|/Game/2_BP/6_UI/PauseMenu/WBP_PauseMenu.WBP_PauseMenu_C|SetAlien _output_get self)
    (Input|SetInputModeGameandUI (Class|GameplayStatics|GetPlayerControllerfromID) 0 "DoNotLock" false false)
    (Variables|/Script/Engine.PlayerController|SetbShowMouseCursor (Class|GameplayStatics|GetPlayerControllerfromID) (Variables|Default|GetPaused))
    (bind _returnvalue_2 (Settings|GetGameUserSettings))
    (Class|PlayerController|SetMouseLocation (Class|GameplayStatics|GetPlayerControllerfromID) (/ (.X (Utilities|Struct|BreakIntPoint (Class|GameUserSettings|GetScreenResolution _returnvalue_2))) 2) (/ (.Y (Utilities|Struct|BreakIntPoint (Class|GameUserSettings|GetScreenResolution _returnvalue_2))) 2))
    (Game|SetGamePaused true)))